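; BP_Slash is a hack-and-slash skill actor that performs a one-shot radial slash attack for its Character.
; On BeginPlay it snaps onto the Character's mesh and applies full radial damage around its own location, ignoring that Character and crediting its controller.
; It also binds to the Attack particle system's finished event, with EventFinishAttack printing a debug string and destroying the actor, so the effect governs its lifetime.
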(event `self.ReceiveBeginPlay`
  (add `NiagaraComponent.OnSystemFinished` (`self.Attack`) (`|CreateDelegate` :!event `EventFinishAttack`))
  (`self.K2_AttachToComponent` (`Character.Mesh` (`self.Character`)) "None" "SnapToTarget" "SnapToTarget" "KeepWorld")
  (`GameplayStatics.ApplyRadialDamage` 10.0 (`self.K2_GetActorLocation`) 200.0 null (`|MakeArray` (`self.Character`) :!type "Actor Object Reference") self (`Pawn.GetController` (`self.Character`)) true))

(fn `EventFinishAttack`
  (params (PSystem :type "NiagaraComponent Object Reference"))
  (`KismetSystemLibrary.PrintString` "EventFinishAttack")
  (`self.K2_DestroyActor`))

(fn `UserConstructionScript`)