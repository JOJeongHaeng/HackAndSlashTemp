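; BP_FireBall is a hack-and-slash skill projectile that flies straight and damages what is around it.
; Tick moves the Ball component along the actor's forward vector at Speed, without sweeping for collision.
; An accumulated timer triggers periodic full radial damage at the Ball's location, ignoring Character and crediting its controller.
; The actor destroys itself after a fixed lifetime rather than on impact.
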(event `self.ReceiveBeginPlay`
  (`KismetSystemLibrary.Delay` 5.0)
  (`self.K2_DestroyActor`))

(event `self.ReceiveTick`
  (params (DeltaSeconds :type "Float (single-precision)"))
  (`|ExecutionSequence`
    (:`then_0`
      (`SceneComponent.K2_AddWorldOffset` (`self.Ball`) (* (* DeltaSeconds (`self.Speed`)) (`self.GetActorForwardVector`)) false false))
    (:`then_1`
      (`self.DoDamage` DeltaSeconds))))

(fn `DoDamage`
  (params (DeltaSeconds :type "Float (double-precision)"))
  (bind _output_get (set `self.DamageDelay` (+ DeltaSeconds (`self.DamageDelay`))))
  (if (> _output_get 0.1)
    (set `self.DamageDelay` 0.0)
    (`GameplayStatics.ApplyRadialDamage` 10.0 (`SceneComponent.K2_GetComponentLocation` (`self.Ball`)) 100.0 null (`|MakeArray` (`self.Character`) :!type "Actor Object Reference") self (`Pawn.GetController` (`self.Character`)) true)))

(fn `UserConstructionScript`)