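; Player state for the hack-and-slash game that holds the character's name and health and announces changes through event dispatchers.
; AddDamage and AddHeal do nothing once HP is at zero; otherwise they update HP and broadcast UpdateHP, and lethal damage also fires Death.
; Healing clamps to a hardcoded 100 rather than MaxHP.
; SetPlayerStat broadcasts the current name and HP values to listeners.
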(fn `AddDamage`
  (params (Damage :type "Float (double-precision)"))
  (if (not (`self.IsDeath`))
    (bind _output_get (set `self.CurHP` (- (`self.CurHP`) Damage)))
    (`self.EventDispatcher_UpdateHP` _output_get (`self.MaxHP`))
    (if (<= (`self.CurHP`) 0.0)
      (`self.EventDispatcher_Death`))))

(fn `AddHeal`
  (params (Heal :type "Float (double-precision)"))
  (if (not (`self.IsDeath`))
    (bind _output_get (set `self.CurHP` (`KismetMathLibrary.FClamp` (+ (`self.CurHP`) Heal) 0.0 100.0)))
    (`self.EventDispatcher_UpdateHP` _output_get (`self.MaxHP`))))

(fn `IsDeath`
  (returns (IsDeath :type Boolean))
  (return (<= (`self.CurHP`) 0.0)))

(fn `SetPlayerStat`
  (`self.EventDispatcher_PlayerStat` (`self.Name`) (`self.MaxHP`) (`self.CurHP`)))

(fn `UserConstructionScript`)