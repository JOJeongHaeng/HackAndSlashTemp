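; Monster stat component that holds a monster's data and current HP in the hack-and-slash game.
; SetMonStat loads a row from DT_Monster by name, starts current HP at MaxHP and broadcasts the stats.
; AddDamage ignores monsters already dead, otherwise subtracts HP without clamping, broadcasts the HP update and fires the death dispatcher when HP reaches zero or below.
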(fn `AddDamage`
  (params (Damage :type "Float (double-precision)"))
  (bind _curmonstat (`self.CurMonStat`))
  (bind (_curmonstat_mondata _curmonstat_curhp) (break `/Game/HackAndSlash/Monster/ST_CurMonster` (`self.CurMonStat`)))
  (if (not (`self.IsDeath`))
    (bind _structout (setmembers `/Game/HackAndSlash/Monster/ST_CurMonster` :`StructRef` _curmonstat :`CurHP` (- _curmonstat_curhp Damage)))
    ; EventDispatcher 호출
    (`self.EventDispatcher_UpdateHP` (`.MaxHP_8_5B39D3C34A1C5719EEFD67AEA3F65888` (break `/Game/HackAndSlash/Monster/ST_Monster` (break `/Game/HackAndSlash/Monster/ST_CurMonster` _structout))) (`.CurHP_5_AEB217F54FD4E4E48D0201A6F004F01B` (break `/Game/HackAndSlash/Monster/ST_CurMonster` _structout)))
    (if (<= (`.CurHP_5_AEB217F54FD4E4E48D0201A6F004F01B` (break `/Game/HackAndSlash/Monster/ST_CurMonster` _curmonstat)) 0.0)
      (`self.EventDispatcher_Death` (`self.CurMonStat`)))))

(fn `IsDeath`
  (returns (IsDeath :type Boolean))
  (bind (_curmonstat_mondata _curmonstat_curhp) (break `/Game/HackAndSlash/Monster/ST_CurMonster` (`self.CurMonStat`)))
  (return (<= _curmonstat_curhp 0.0)))

(fn `SetMonStat`
  (params (RowName :type Name))
  (bind _returnvalue (`|GetDataTableRow` "/Game/HackAndSlash/Monster/DT_Monster.DT_Monster" RowName)
    (:`then`
      (bind _output_get (set `self.CurMonStat` (make `/Game/HackAndSlash/Monster/ST_CurMonster` _returnvalue (`.MaxHP_8_5B39D3C34A1C5719EEFD67AEA3F65888` (break `/Game/HackAndSlash/Monster/ST_Monster` _returnvalue)))))
      (`self.EventDispatcher_MonStat` _output_get))))