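; BP_HUDCoin is the HUD for a coin game, showing the coin value, game time in seconds and game state.
; On BeginPlay it creates the HudWidgetCoin widget and binds to event dispatchers on BP_GameStateCoin and the first player's BP_PlayerStateCoin.
; Update functions forward values to the widget, keeping it event-driven, and the current game state is pushed once after binding.
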(event `self.ReceiveBeginPlay`
  (bind _returnvalue (`|CreateWidget` "/Game/BluePrint/HudWidgetCoin.HudWidgetCoin_C"))
  (bind _output_get (set `self.HudWidget` _returnvalue))
  (`UserWidget.AddToViewport` _output_get 0)
  (`self.BindGameState`)
  (bind _asbp_player_state_coin (cast `/Game/BluePrint/BP_PlayerStateCoin` (`Controller.PlayerState` (`GameplayStatics.GetPlayerController` 0))))
  (add `/Game/BluePrint/BP_PlayerStateCoin.EventDispatcher_AddCoin` _asbp_player_state_coin (`|CreateDelegate` :!event `UpdateCoin`)))

(fn `BindGameState`
  (bind _asbp_game_state (cast `/Game/BluePrint/BP_GameStateCoin` (`GameplayStatics.GetGameState`)))
  (add `/Game/BluePrint/BP_GameStateCoin.EventDispatcher_TotalSec` _asbp_game_state (`|CreateDelegate` :!event `UpdateTotalGameSec`))
  (add `/Game/BluePrint/BP_GameStateCoin.EventDispatcher_ChangeGameState` _asbp_game_state (`|CreateDelegate` :!event `UpdateGameState`))
  (`self.UpdateGameState` (`/Game/BluePrint/BP_GameStateCoin.GameState` _asbp_game_state)))

(fn `UpdateCoin`
  (params (Coin :type Integer))
  (`/Game/BluePrint/HudWidgetCoin.UpdateCoin` (`self.HudWidget`) Coin))

(fn `UpdateGameState`
  (params (NewParam :type "/Game/BluePrint/EN_GameState Enum" :default "NewEnumerator0"))
  (`/Game/BluePrint/HudWidgetCoin.UpdateGameState` (`self.HudWidget`) NewParam))

(fn `UpdateTotalGameSec`
  (params (TotalSec :type "Float (double-precision)"))
  (`/Game/BluePrint/HudWidgetCoin.UpdateTotalSec` (`self.HudWidget`) TotalSec))

(fn `UserConstructionScript`)