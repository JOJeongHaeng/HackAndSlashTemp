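; BP_GameStateCoin holds the current game state and an elapsed-time counter, presumably for a coin game.
; On Tick it accumulates delta time during Ready and Play and broadcasts the running total through an event dispatcher.
; ChangeGameState stores the new state, prints its name and broadcasts the change through a second dispatcher.
; ResetTime zeroes the counter without broadcasting, and changing state does not reset it.
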(event `self.ReceiveTick`
  (params (DeltaSeconds :type "Float (single-precision)"))
  (switch `/Game/BluePrint/EN_GameState` (`self.GameState`)
    (:`NewEnumerator1`
      _)
    (:`NewEnumerator2`
      _))
  (bind _output_get (set `self.TotalDeltaSeconds` (+ DeltaSeconds (`self.TotalDeltaSeconds`))))
  (`self.EventDispatcher_TotalSec` _output_get))

(fn `ChangeGameState`
  (params (GameState :type "/Game/BluePrint/EN_GameState Enum" :default "NewEnumerator0"))
  (bind _output_get (set `self.GameState` GameState))
  (`KismetSystemLibrary.PrintString` (`|GetEnumeratorNameAsString` _output_get))
  (`self.EventDispatcher_ChangeGameState` _output_get))

(fn `ResetTime`
  (set `self.TotalDeltaSeconds` 0.0))

(fn `UserConstructionScript`)